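; Trapdoor floor obstacle that swings open when the player stands on it and can be frozen by a time-freeze ability.
; Box overlap starts a timer that plays a Timeline pitching the Plane open; leaving cancels the timer and reverses it.
; Freezing stops the Timeline and blocks new triggers for a fixed delay, without resuming it afterward; rewinding is unsupported.
; Custom depth stencil values mark aimed and frozen states.
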(event `self.Box.OnComponentBeginOverlap`
  (params (OverlappedComponent :type "PrimitiveComponent Object Reference") (OtherActor :type "Actor Object Reference") (OtherComp :type "PrimitiveComponent Object Reference") (OtherBodyIndex :type Integer) (bFromSweep :type Boolean) (SweepResult :type "HitResult Structure (by ref)"))
  (if (and (== OtherActor (`GameplayStatics.GetPlayerCharacter` 0)) (not (`self.IsOverlap`)))
    (set `self.IsOverlap` true)
    (if (not (`self.IsFreezing`))
      (bind _returnvalue (`KismetSystemLibrary.K2_SetTimerDelegate` (delegate `TrapdoorOpening`) (`self.TrapOpeningTime`)))
      (set `self.Timer` _returnvalue))))

(event `TrapdoorOpening`
  (bind (_direction _opentrap) (`Timeline|Timeline`)
    (:`Update`
      (`SceneComponent.K2_SetRelativeRotation` (`self.Plane`) (`KismetMathLibrary.MakeRotator` 0.0 (`KismetMathLibrary.Lerp` 0.0 90.0 _opentrap)) false false))))

(event `self.Box.OnComponentEndOverlap`
  (params (OverlappedComponent :type "PrimitiveComponent Object Reference") (OtherActor :type "Actor Object Reference") (OtherComp :type "PrimitiveComponent Object Reference") (OtherBodyIndex :type Integer))
  (if (`self.IsFreezing`)
    _
    (elif (== OtherActor (`GameplayStatics.GetPlayerCharacter` 0))
      (`KismetSystemLibrary.K2_ClearAndInvalidateTimerHandle` (`self.Timer`))
      (`TimelineComponent.Reverse` (`self.Timeline`))
      (set `self.IsOverlap` false))))

(event `/Game/WMTOY_Contents/Interfaces/BPI_Aimed.Aimed`
  (if (not (`self.IsFreezing`))
    (`PrimitiveComponent.SetCustomDepthStencilValue` (`self.Plane`) 1)))

(event `/Game/WMTOY_Contents/Interfaces/BPI_ClearAim.ClearAim`
  (if (not (`self.IsFreezing`))
    (`PrimitiveComponent.SetCustomDepthStencilValue` (`self.Plane`) 0)))

(event `/Game/WMTOY_Contents/Interfaces/BPI_TimeFreezing.TimeFreezing`
  (set `self.IsFreezing` true)
  (`PrimitiveComponent.SetCustomDepthStencilValue` (`self.Plane`) 2)
  (`TimelineComponent.Stop` (`self.Timeline`))
  (`KismetSystemLibrary.Delay` 3.0)
  (set `self.IsFreezing` false)
  (`PrimitiveComponent.SetCustomDepthStencilValue` (`self.Plane`) 0))

(fn `CanFreezing`
  (returns (CanFreezing :type Boolean))
  (return true))

(fn `CanRewinding`
  (returns (CanRewinding :type Boolean))
  (return false))

(fn `GetFreezingState`
  (returns (IsFreezing :type Boolean))
  (return (`self.IsFreezing`)))

(fn `UserConstructionScript`)