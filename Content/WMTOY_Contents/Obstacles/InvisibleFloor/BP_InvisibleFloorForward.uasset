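; Invisible floor obstacle that is revealed only while the player's time gauge is high enough.
; It hides its cube on BeginPlay, then every Tick reads the ChronoHacker player's TimeGauge against a fixed threshold to toggle cube visibility and a Niagara grid effect.
; Only visibility changes, with collision left untouched.
; Its freeze and rewind query functions all return false, opting it out of those time powers.
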(event `self.ReceiveBeginPlay`
  (`SceneComponent.SetVisibility` (`self.Cube`) false false))

(event `self.ReceiveTick`
  (params (DeltaSeconds :type "Float (single-precision)"))
  (bind _asbp_chrono_hacker (cast `/Game/WMTOY_Contents/Character/BP_ChronoHacker` (`GameplayStatics.GetPlayerCharacter` 0)))
  (bind (_mystat_maxhp _mystat_curhp _mystat_timegauge) (break `/Game/WMTOY_Contents/Character/ST_Stats` (`/Game/WMTOY_Contents/Character/BP_ChronoHacker.MyStat` _asbp_chrono_hacker)))
  (if (>= _mystat_timegauge 60.0)
    (`SceneComponent.SetVisibility` (`self.Cube`) true false)
    (`ActorComponent.SetActive` (`self.NS_GridFigure`) true false)
    (else
      (`SceneComponent.SetVisibility` (`self.Cube`) false false)
      (`ActorComponent.SetActive` (`self.NS_GridFigure`) false false))))

(fn `CanFreezing`
  (returns (CanFreezing :type Boolean))
  (return false))

(fn `CanRewinding`
  (returns (CanRewinding :type Boolean))
  (return false))

(fn `GetFreezingState`
  (returns (IsFreezing :type Boolean))
  (return false))

(fn `UserConstructionScript`)