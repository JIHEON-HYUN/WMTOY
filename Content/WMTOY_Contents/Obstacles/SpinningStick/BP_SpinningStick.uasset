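; BP_SpinningStick is an obstacle that spins continuously and responds to time freeze and rewind skills.
; A looping timer steps the Stick's yaw by SpinSpeed.
; TimeRewinding reverses one step and activates NSRewinding; the flag clears each tick, so sustained rewind needs repeated calls.
; TimeFreezing clears the timer for three seconds, blocking rewind and aim changes, while custom-depth stencil values mark aimed and frozen states.
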(event `self.ReceiveBeginPlay`
  ;[1 1 1] 정방향인지 TimeRewinding 중인지 판단 후, Floor/Blade 회전 반복
  (`self.RotateStick`))

(event `RotateStick`
  ;[1 1 1] 정방향인지 TimeRewinding 중인지 판단 후, Floor/Blade 회전 반복
  (bind _returnvalue (`KismetSystemLibrary.K2_SetTimerDelegate` (delegate `Rotate`) 0.01 true))
  (set `self.RotationLoop` _returnvalue))

(event `Rotate`
  (bind (_returnvalue_roll _returnvalue_pitch _returnvalue_yaw) (`KismetMathLibrary.BreakRotator` (`SceneComponent.K2_GetComponentRotation` (`self.Stick`))))
  (bind (_returnvalue_roll_2 _returnvalue_pitch_2 _returnvalue_yaw_2) (`KismetMathLibrary.BreakRotator` (`SceneComponent.K2_GetComponentRotation` (`self.Stick`))))
  ;[1 1 1] 정방향인지 TimeRewinding 중인지 판단 후, Floor/Blade 회전 반복
  (if (`self.IsRewinding`)
    (`SceneComponent.K2_SetRelativeRotation` (`self.Stick`) (`KismetMathLibrary.MakeRotator` _returnvalue_roll_2 _returnvalue_pitch_2 (+ _returnvalue_yaw_2 (* (`self.SpinSpeed`) -1.0))) false false)
    (set `self.IsRewinding` false)
    (`ActorComponent.SetActive` (`self.NS_Rewinding`) false false)
    (else
      (`SceneComponent.K2_SetRelativeRotation` (`self.Stick`) (`KismetMathLibrary.MakeRotator` _returnvalue_roll _returnvalue_pitch (+ _returnvalue_yaw (`self.SpinSpeed`))) false false))))

(event `self.TimeRewinding`
  ;[1 1 1] Aim, TimeFreezing, TimeRewinding 구현
  (if (not (`self.IsFreezing`))
    (set `self.IsRewinding` true)
    (`ActorComponent.SetActive` (`self.NS_Rewinding`) true false)))

(event `self.Aimed`
  ;[1 1 1] Aim, TimeFreezing, TimeRewinding 구현
  (if (not (`self.IsFreezing`))
    (`PrimitiveComponent.SetCustomDepthStencilValue` (`self.Stick`) 1)))

(event `self.ClearAim`
  ;[1 1 1] Aim, TimeFreezing, TimeRewinding 구현
  (if (not (`self.IsFreezing`))
    (`PrimitiveComponent.SetCustomDepthStencilValue` (`self.Stick`) 0)))

(event `self.TimeFreezing`
  ;[1 1 1] Aim, TimeFreezing, TimeRewinding 구현
  (set `self.IsFreezing` true)
  (`PrimitiveComponent.SetCustomDepthStencilValue` (`self.Stick`) 2)
  (`KismetSystemLibrary.K2_ClearAndInvalidateTimerHandle` (`self.RotationLoop`))
  (`KismetSystemLibrary.Delay` 3.0)
  (`self.RotateStick`)
  (`PrimitiveComponent.SetCustomDepthStencilValue` (`self.Stick`) 0)
  (set `self.IsFreezing` false))

(fn `CanFreezing`
  (returns (CanFreezing :type Boolean))
  (return true))

(fn `CanRewinding`
  (returns (CanRewinding :type Boolean))
  (return true))

(fn `GetFreezingState`
  (returns (IsFreezing :type Boolean))
  (return (`self.IsFreezing`)))

(fn `GetRewindingState`
  (returns (IsRewinding :type Boolean))
  (return (`self.IsRewinding`)))

(fn `UserConstructionScript`)