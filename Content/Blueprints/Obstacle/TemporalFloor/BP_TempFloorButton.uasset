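; BP_TempFloorButton is an obstacle button that triggers the temporal floors listed in its TargetFloor array.
; Overlapping its Box hides the Sphere mesh, disables the Box collision and calls PressedButton on each target floor.
; After a short delay it restores visibility and collision and clears the IsOverlap guard, so the button can be triggered again.
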(event `self.Box.OnComponentBeginOverlap`
  (params (OverlappedComponent :type "PrimitiveComponent Object Reference") (OtherActor :type "Actor Object Reference") (OtherComp :type "PrimitiveComponent Object Reference") (OtherBodyIndex :type Integer) (bFromSweep :type Boolean) (SweepResult :type "HitResult Structure (by ref)"))
  (if (not (`self.IsOverlap`))
    (set `self.IsOverlap` true)
    (`SceneComponent.SetVisibility` (`self.Sphere`) false false)
    (`PrimitiveComponent.SetCollisionEnabled` (`self.Box`) "NoCollision")
    (for _array_element (`self.TargetFloor`)
      (`/Game/Blueprints/Obstacle/TemporalFloor/BP_TempFloor.PressedButton` _array_element))
    (`KismetSystemLibrary.Delay` 3.0)
    (`SceneComponent.SetVisibility` (`self.Sphere`) true false)
    (`PrimitiveComponent.SetCollisionEnabled` (`self.Box`) "QueryAndPhysics")
    (set `self.IsOverlap` false)))

(fn `UserConstructionScript`)