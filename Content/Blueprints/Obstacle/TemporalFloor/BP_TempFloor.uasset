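; BP_TempFloor is a temporary floor obstacle that starts hidden and non-collidable, becoming solid for a few seconds when a button press triggers it.
; Tick applies visibility and collision from IsActive, which PressedButton sets and ReleasedButton clears after a delay.
; TimeFreezing extends that window with a second delay if still set when the first ends.
; Custom depth stencil values mark aimed and frozen states, with frozen overriding aim changes.
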(event `self.ReceiveBeginPlay`
  (bind _cube (`self.Cube`))
  (`SceneComponent.SetVisibility` _cube false false)
  (`PrimitiveComponent.SetCollisionEnabled` _cube "NoCollision"))

(event `self.ReceiveTick`
  (params (DeltaSeconds :type "Float (single-precision)"))
  (if (`self.IsActive`)
    (`SceneComponent.SetVisibility` (`self.Cube`) true false)
    (`PrimitiveComponent.SetCollisionEnabled` (`self.Cube`) "QueryAndPhysics")
    (else
      (`SceneComponent.SetVisibility` (`self.Cube`) false false)
      (`PrimitiveComponent.SetCollisionEnabled` (`self.Cube`) "NoCollision"))))

(event `/Game/Blueprints/Interfaces/BPI_Aimed.Aimed`
  (if (not (`self.IsFreezing`))
    (`PrimitiveComponent.SetCustomDepthStencilValue` (`self.Cube`) 1)))

(event `/Game/Blueprints/Interfaces/BPI_ClearAim.ClearAim`
  (if (not (`self.IsFreezing`))
    (`PrimitiveComponent.SetCustomDepthStencilValue` (`self.Cube`) 0)))

(event `PressedButton`
  (set `self.IsActive` true)
  (`KismetSystemLibrary.Delay` 3.0)
  (if (`self.IsFreezing`)
    (`KismetSystemLibrary.Delay` 3.0)
    (`PrimitiveComponent.SetCustomDepthStencilValue` (`self.Cube`) 0))
  (`self.ReleasedButton`))

(event `ReleasedButton`
  (set `self.IsActive` false)
  (set `self.IsFreezing` false))

(event `/Game/Blueprints/Interfaces/BPI_TimeFreezing.TimeFreezing`
  (set `self.IsFreezing` true)
  (`PrimitiveComponent.SetCustomDepthStencilValue` (`self.Cube`) 2))

(fn `UserConstructionScript`)