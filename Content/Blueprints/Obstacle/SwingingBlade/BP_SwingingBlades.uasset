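; Swinging blade obstacle that knocks back the ChronoHacker player on box overlap and can be time-frozen.
; With UseRotation set, it zeroes RotatingMovement and ping-pongs a timeline that lerps the cylinder's yaw across a half-circle arc.
; TimeFreezing briefly stops rotation updates, flipping the timeline direction on each update to hold the swing in place.
; Custom depth stencil values on the axe mesh mark aimed and frozen states.
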(event `self.ReceiveBeginPlay`
  (if (`self.UseRotation`)
    (`TimelineComponent.SetTimelineLength` (`self.Timeline`) (`self.SwingSpeed`))
    (`self.PlayAxeswing`) ; starts event
    (set `RotatingMovementComponent.RotationRate` (struct) (`self.RotatingMovement`))))

(event `PlayAxeswing`
  (set `self.Direction` "Forward")
  (bind (_direction _swingtimeline) (`Timeline|Timeline` :!label _label)
    (:`Update`
      (if (`self.IsFreezing`)
        (if (`|EnumEquality` _direction "Forward") :!label _label_2
          (`self.ReverseSwing`)
          (else
            (`self.PlayAxeswing`)))
        (else
          (`SceneComponent.K2_SetRelativeRotation` (`self.Cylinder`) (`KismetMathLibrary.MakeRotator` 0.0 0.0 (`KismetMathLibrary.Lerp` -90.0 90.0 _swingtimeline)) false false))))
    (:`Finished`
      (goto _label_2))))

(event `ReverseSwing`
  (set `self.Direction` "Backward")
  (goto _label :!via `Reverse`))

(event `self.Box.OnComponentBeginOverlap`
  (params (OverlappedComponent :type "PrimitiveComponent Object Reference") (OtherActor :type "Actor Object Reference") (OtherComp :type "PrimitiveComponent Object Reference") (OtherBodyIndex :type Integer) (bFromSweep :type Boolean) (SweepResult :type "HitResult Structure (by ref)"))
  (if (== OtherActor (`GameplayStatics.GetPlayerCharacter` 0))
    (if (not (`self.Death`))
      (bind _asbp_chrono_hacker (cast `/Game/Blueprints/Character/BP_ChronoHacker` (`GameplayStatics.GetPlayerCharacter` 0)))
      (`/Game/Blueprints/Character/BP_ChronoHacker.KnockBack` _asbp_chrono_hacker (`self.KnockBackAmount`)))))

(event `/Game/Blueprints/Interfaces/BPI_TimeFreezing.TimeFreezing`
  (set `self.IsFreezing` true)
  (`PrimitiveComponent.SetCustomDepthStencilValue` (`self.AxeMesh`) 2)
  (`KismetSystemLibrary.Delay` 3.0)
  (set `self.IsFreezing` false)
  (`PrimitiveComponent.SetCustomDepthStencilValue` (`self.AxeMesh`) 0))

(event `/Game/Blueprints/Interfaces/BPI_Aimed.Aimed`
  (if (not (`self.IsFreezing`))
    (`PrimitiveComponent.SetCustomDepthStencilValue` (`self.AxeMesh`) 1)))

(event `/Game/Blueprints/Interfaces/BPI_ClearAim.ClearAim`
  (if (not (`self.IsFreezing`))
    (`PrimitiveComponent.SetCustomDepthStencilValue` (`self.AxeMesh`) 0)))

(fn `UserConstructionScript`)