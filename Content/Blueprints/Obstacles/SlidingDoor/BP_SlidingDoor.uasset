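; Sliding door obstacle that endlessly opens and closes two panels, damaging actors that overlap either door's box.
; A Timeline lerps both panels apart and reverses on each finish to loop.
; Time freezing pauses panel movement for three seconds while the Timeline keeps running, and rewinding is unsupported.
; Custom depth stencil values mark aimed and frozen states, and damage is skipped during freeze or slowed global time.
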(event `self.ReceiveBeginPlay`
  ;[1 1 1] Timeline에 따라서 문이 열리고 닫히고 반복
  (`self.Open`))

(event `Open`
  ;[1 1 1] Timeline에 따라서 문이 열리고 닫히고 반복
  (set `self.Direction` "Forward")
  (bind (_direction _doortrack) (`Timeline|Timeline` :!label _label)
    (:`Update`
      (if (not (`self.IsFreezing`))
        (`SceneComponent.K2_SetRelativeLocation` (`self.LeftDoor`) (`KismetMathLibrary.MakeVector` (`KismetMathLibrary.Lerp` -76.0 -200.0 _doortrack)) false false)
        (`SceneComponent.K2_SetRelativeLocation` (`self.RightDoor`) (`KismetMathLibrary.MakeVector` (`KismetMathLibrary.Lerp` 76.0 200.0 _doortrack)) false false)))
    (:`Finished`
      (if (`|EnumEquality` _direction "Forward")
        (`self.Close`)
        (else
          (`self.Open`))))))

(event `Close`
  ;[1 1 1] Timeline에 따라서 문이 열리고 닫히고 반복
  (set `self.Direction` "Backward")
  (goto _label :!via `Reverse`))

(event `/Game/Blueprints/Interfaces/BPI_TimeFreezing.TimeFreezing`
  ;[1 1 1] Aim, TimeFreezing 구현
  (set `self.IsFreezing` true)
  (`PrimitiveComponent.SetCustomDepthStencilValue` (`self.LeftDoor`) 2)
  (`PrimitiveComponent.SetCustomDepthStencilValue` (`self.RightDoor`) 2)
  (`KismetSystemLibrary.Delay` 3.0)
  (set `self.IsFreezing` false)
  (`PrimitiveComponent.SetCustomDepthStencilValue` (`self.LeftDoor`) 0)
  (`PrimitiveComponent.SetCustomDepthStencilValue` (`self.RightDoor`) 0))

(event `/Game/Blueprints/Interfaces/BPI_Aimed.Aimed`
  ;[1 1 1] Aim, TimeFreezing 구현
  (if (not (`self.IsFreezing`))
    (`PrimitiveComponent.SetCustomDepthStencilValue` (`self.LeftDoor`) 1)
    (`PrimitiveComponent.SetCustomDepthStencilValue` (`self.RightDoor`) 1)))

(event `/Game/Blueprints/Interfaces/BPI_ClearAim.ClearAim`
  ;[1 1 1] Aim, TimeFreezing 구현
  (if (not (`self.IsFreezing`))
    (`PrimitiveComponent.SetCustomDepthStencilValue` (`self.LeftDoor`) 0)
    (`PrimitiveComponent.SetCustomDepthStencilValue` (`self.RightDoor`) 0)))

(event `self.LeftDoorBox.OnComponentBeginOverlap`
  (params (OverlappedComponent :type "PrimitiveComponent Object Reference") (OtherActor :type "Actor Object Reference") (OtherComp :type "PrimitiveComponent Object Reference") (OtherBodyIndex :type Integer) (bFromSweep :type Boolean) (SweepResult :type "HitResult Structure (by ref)"))
  ;[1 1 1] 데미지 이벤트 (시간 감속, TimeFreezing 상태에서는 데미지 X)
  (if (and (>= (`GameplayStatics.GetGlobalTimeDilation`) 1.0) (not (`self.IsFreezing`)))
    (`GameplayStatics.ApplyDamage` OtherActor 100.0 null null "/Script/Engine.DamageType")))

(event `self.RightDoorBox.OnComponentBeginOverlap`
  (params (OverlappedComponent :type "PrimitiveComponent Object Reference") (OtherActor :type "Actor Object Reference") (OtherComp :type "PrimitiveComponent Object Reference") (OtherBodyIndex :type Integer) (bFromSweep :type Boolean) (SweepResult :type "HitResult Structure (by ref)"))
  ;[1 1 1] 데미지 이벤트 (시간 감속, TimeFreezing 상태에서는 데미지 X)
  (if (and (>= (`GameplayStatics.GetGlobalTimeDilation`) 1.0) (not (`self.IsFreezing`)))
    (`GameplayStatics.ApplyDamage` OtherActor 100.0 null null "/Script/Engine.DamageType")))

(fn `CanFreezing`
  (returns (CanFreezing :type Boolean))
  (return true))

(fn `CanRewinding`
  (returns (CanRewinding :type Boolean))
  (return false))

(fn `GetFreezingState`
  (returns (IsFreezing :type Boolean))
  (return (`self.IsFreezing`)))

(fn `UserConstructionScript`)