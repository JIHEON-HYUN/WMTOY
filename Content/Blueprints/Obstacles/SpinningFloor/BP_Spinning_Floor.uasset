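; Spinning floor obstacle whose Floor and Blade counter-rotate on a looping timer and that reacts to the player's time skills.
; Rewind reverses one tick per call, while freeze clears the timer for a few seconds before restarting it.
; Custom depth stencil values mark aimed and frozen states.
; Box overlap always knocks back BP_ChronoHacker, but damages only when unfrozen and not slowed, hitting harder when global time is sped up.
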(event `self.ReceiveBeginPlay`
  ;[1 1 1] 정방향인지 TimeRewinding 중인지 판단 후, Floor/Blade 회전 반복
  (`self.RotateFloor`))

(event `RotateFloor`
  ;[1 1 1] 정방향인지 TimeRewinding 중인지 판단 후, Floor/Blade 회전 반복
  (bind _returnvalue (`KismetSystemLibrary.K2_SetTimerDelegate` (delegate `Rotate`) 0.01 true))
  (set `self.RotationLoop` _returnvalue))

(event `Rotate`
  (bind (_returnvalue_roll _returnvalue_pitch _returnvalue_yaw) (`KismetMathLibrary.BreakRotator` (`SceneComponent.K2_GetComponentRotation` (`self.Blade`))))
  (bind (_returnvalue_roll_2 _returnvalue_pitch_2 _returnvalue_yaw_2) (`KismetMathLibrary.BreakRotator` (`SceneComponent.K2_GetComponentRotation` (`self.Floor`))))
  (bind (_returnvalue_roll_3 _returnvalue_pitch_3 _returnvalue_yaw_3) (`KismetMathLibrary.BreakRotator` (`SceneComponent.K2_GetComponentRotation` (`self.Blade`))))
  (bind (_returnvalue_roll_4 _returnvalue_pitch_4 _returnvalue_yaw_4) (`KismetMathLibrary.BreakRotator` (`SceneComponent.K2_GetComponentRotation` (`self.Floor`))))
  ;[1 1 1] 정방향인지 TimeRewinding 중인지 판단 후, Floor/Blade 회전 반복
  (if (`self.IsRewinding`)
    (`SceneComponent.K2_SetRelativeRotation` (`self.Floor`) (`KismetMathLibrary.MakeRotator` _returnvalue_roll_4 _returnvalue_pitch_4 (+ _returnvalue_yaw_4 -2.0)) false false)
    (`SceneComponent.K2_SetRelativeRotation` (`self.Blade`) (`KismetMathLibrary.MakeRotator` _returnvalue_roll _returnvalue_pitch (- _returnvalue_yaw -1.0)) false false)
    (set `self.IsRewinding` false)
    (else
      (`SceneComponent.K2_SetRelativeRotation` (`self.Floor`) (`KismetMathLibrary.MakeRotator` _returnvalue_roll_2 _returnvalue_pitch_2 (+ _returnvalue_yaw_2 2.0)) false false)
      (`SceneComponent.K2_SetRelativeRotation` (`self.Blade`) (`KismetMathLibrary.MakeRotator` _returnvalue_roll_3 _returnvalue_pitch_3 (- _returnvalue_yaw_3 1.0)) false false))))

(event `/Game/Blueprints/Interfaces/BPI_TimeRewinding.TimeRewinding`
  ;[1 1 1] Aim, TimeFreezing, TimeRewinding 구현
  (set `self.IsRewinding` true))

(event `/Game/Blueprints/Interfaces/BPI_Aimed.Aimed`
  ;[1 1 1] Aim, TimeFreezing, TimeRewinding 구현
  (if (not (`self.IsFreezing`))
    (`PrimitiveComponent.SetCustomDepthStencilValue` (`self.Floor`) 1)
    (`PrimitiveComponent.SetCustomDepthStencilValue` (`self.Middle`) 1)
    (`PrimitiveComponent.SetCustomDepthStencilValue` (`self.Blade`) 1)))

(event `/Game/Blueprints/Interfaces/BPI_ClearAim.ClearAim`
  ;[1 1 1] Aim, TimeFreezing, TimeRewinding 구현
  (if (not (`self.IsFreezing`))
    (`PrimitiveComponent.SetCustomDepthStencilValue` (`self.Floor`) 0)
    (`PrimitiveComponent.SetCustomDepthStencilValue` (`self.Middle`) 0)
    (`PrimitiveComponent.SetCustomDepthStencilValue` (`self.Blade`) 0)))

(event `/Game/Blueprints/Interfaces/BPI_TimeFreezing.TimeFreezing`
  ;[1 1 1] Aim, TimeFreezing, TimeRewinding 구현
  (set `self.IsFreezing` true)
  (`PrimitiveComponent.SetCustomDepthStencilValue` (`self.Floor`) 2)
  (`PrimitiveComponent.SetCustomDepthStencilValue` (`self.Middle`) 2)
  (`PrimitiveComponent.SetCustomDepthStencilValue` (`self.Blade`) 2)
  (`KismetSystemLibrary.K2_ClearAndInvalidateTimerHandle` (`self.RotationLoop`))
  (`KismetSystemLibrary.Delay` 3.0)
  (`self.RotateFloor`)
  (`PrimitiveComponent.SetCustomDepthStencilValue` (`self.Floor`) 0)
  (`PrimitiveComponent.SetCustomDepthStencilValue` (`self.Middle`) 0)
  (`PrimitiveComponent.SetCustomDepthStencilValue` (`self.Blade`) 0)
  (set `self.IsFreezing` false))

(event `self.Box.OnComponentBeginOverlap`
  (params (OverlappedComponent :type "PrimitiveComponent Object Reference") (OtherActor :type "Actor Object Reference") (OtherComp :type "PrimitiveComponent Object Reference") (OtherBodyIndex :type Integer) (bFromSweep :type Boolean) (SweepResult :type "HitResult Structure (by ref)"))
  ;[1 1 1] 넉백 후 데미지 이벤트 (시간 감속, TimeFreezing 상태에서는 데미지 X)
  (bind _asbp_chrono_hacker (cast `/Game/Blueprints/Character/BP_ChronoHacker` OtherActor))
  (`/Game/Blueprints/Character/BP_ChronoHacker.KnockBack` _asbp_chrono_hacker (`self.Knock Back Value`) (`self.K2_GetActorLocation`))
  (if (and (>= (`GameplayStatics.GetGlobalTimeDilation`) 1.0) (not (`self.IsFreezing`)))
    (if (> (`GameplayStatics.GetGlobalTimeDilation`) 1.0)
      (`GameplayStatics.ApplyDamage` _asbp_chrono_hacker 100.0 null null "/Script/Engine.DamageType")
      (else
        (`GameplayStatics.ApplyDamage` _asbp_chrono_hacker 30.0 null null "/Script/Engine.DamageType")))))

(fn `UserConstructionScript`)