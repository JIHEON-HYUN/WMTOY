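; Swinging blade obstacle that knocks back and damages BP_ChronoHacker on overlap and reacts to time skills.
; A Timeline ping-pongs the cylinder's yaw when UseRotation is set.
; TimeFreezing halts rotation temporarily, custom-depth stencils mark frozen and aimed states, and TimeRewinding briefly flips swing direction.
; Knockback always applies, while damage is skipped when frozen or slowed and increases when global time is sped up.
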(event `self.ReceiveBeginPlay`
  ;[1 1 1] Timeline에 따라 스윙 반복
  (if (`self.UseRotation`)
    (`TimelineComponent.SetTimelineLength` (`self.Timeline`) (`self.SwingInterval`))
    (`self.PlayAxeswing`) ; starts event
    (set `RotatingMovementComponent.RotationRate` (struct) (`self.RotatingMovement`))))

(event `PlayAxeswing`
  ;[1 1 1] Timeline에 따라 스윙 반복
  (set `self.Direction` "Forward")
  (bind (_direction _swingtimeline) (`Timeline|Timeline` :!label _label)
    (:`Update`
      (if (`self.IsFreezing`)
        (if (`|EnumEquality` _direction "Forward") :!label _label_2
          (`self.ReverseSwing`)
          (else
            (`self.PlayAxeswing`)))
        (else
          (`SceneComponent.K2_SetRelativeRotation` (`self.Cylinder`) (`KismetMathLibrary.MakeRotator` 0.0 0.0 (`KismetMathLibrary.Lerp` -90.0 90.0 _swingtimeline)) false false))))
    (:`Finished`
      (goto _label_2))))

(event `ReverseSwing`
  ;[1 1 1] Timeline에 따라 스윙 반복
  (set `self.Direction` "Backward")
  (goto _label :!via `Reverse`))

(event `/Game/Blueprints/Interfaces/BPI_TimeFreezing.TimeFreezing`
  ;[1 1 1] Aim, TimeFreezing, TimeRewinding 구현
  (set `self.IsFreezing` true)
  (`PrimitiveComponent.SetCustomDepthStencilValue` (`self.Cylinder`) 2)
  (`PrimitiveComponent.SetCustomDepthStencilValue` (`self.AxeMesh`) 2)
  (`KismetSystemLibrary.Delay` 3.0)
  (set `self.IsFreezing` false)
  (`PrimitiveComponent.SetCustomDepthStencilValue` (`self.Cylinder`) 0)
  (`PrimitiveComponent.SetCustomDepthStencilValue` (`self.AxeMesh`) 0))

(event `/Game/Blueprints/Interfaces/BPI_Aimed.Aimed`
  ;[1 1 1] Aim, TimeFreezing, TimeRewinding 구현
  (if (not (`self.IsFreezing`))
    (`PrimitiveComponent.SetCustomDepthStencilValue` (`self.Cylinder`) 1)
    (`PrimitiveComponent.SetCustomDepthStencilValue` (`self.AxeMesh`) 1)))

(event `/Game/Blueprints/Interfaces/BPI_ClearAim.ClearAim`
  ;[1 1 1] Aim, TimeFreezing, TimeRewinding 구현
  (if (not (`self.IsFreezing`))
    (`PrimitiveComponent.SetCustomDepthStencilValue` (`self.Cylinder`) 0)
    (`PrimitiveComponent.SetCustomDepthStencilValue` (`self.AxeMesh`) 0)))

(event `/Game/Blueprints/Interfaces/BPI_TimeRewinding.TimeRewinding`
  ;[1 1 1] Aim, TimeFreezing, TimeRewinding 구현
  (if (`|EnumEquality` (`self.Direction`) "Forward")
    (`self.ReverseSwing`)
    (`KismetSystemLibrary.Delay` 0.0001)
    (`self.PlayAxeswing`)
    (else
      (`self.PlayAxeswing`)
      (`KismetSystemLibrary.Delay` 0.0001)
      (`self.ReverseSwing`))))

(event `self.Box.OnComponentBeginOverlap`
  (params (OverlappedComponent :type "PrimitiveComponent Object Reference") (OtherActor :type "Actor Object Reference") (OtherComp :type "PrimitiveComponent Object Reference") (OtherBodyIndex :type Integer) (bFromSweep :type Boolean) (SweepResult :type "HitResult Structure (by ref)"))
  ;[1 1 1] 넉백 후 데미지 이벤트 (시간 감속, TimeFreezing 상태에서는 데미지 X)
  (bind _asbp_chrono_hacker (cast `/Game/Blueprints/Character/BP_ChronoHacker` OtherActor))
  (`/Game/Blueprints/Character/BP_ChronoHacker.KnockBack` _asbp_chrono_hacker (`self.KnockBackAmount`) (`self.K2_GetActorLocation`))
  (if (and (>= (`GameplayStatics.GetGlobalTimeDilation`) 1.0) (not (`self.IsFreezing`)))
    (if (> (`GameplayStatics.GetGlobalTimeDilation`) 1.0)
      (`GameplayStatics.ApplyDamage` _asbp_chrono_hacker 100.0 null null "/Script/Engine.DamageType")
      (else
        (`GameplayStatics.ApplyDamage` _asbp_chrono_hacker 20.0 null null "/Script/Engine.DamageType")))))

(fn `UserConstructionScript`)