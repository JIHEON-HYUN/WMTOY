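; TimeTester is a continuously rolling test obstacle that responds to aim, time-freeze and time-rewind events.
; Tick spins it and records location and rotation snapshots at fixed intervals into a capped history, dropping the oldest.
; Each rewind call restores and pops the newest snapshot; with an empty history, IsRewinding stays true, halting spin and recording.
; Freezing pauses Tick for a few seconds, while custom depth stencil values mark aimed and frozen states.
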(event `self.ReceiveTick`
  (params (DeltaSeconds :type "Float (single-precision)"))
  (bind (_returnvalue_roll _returnvalue_pitch _returnvalue_yaw) (`KismetMathLibrary.BreakRotator` (`self.K2_GetActorRotation`)))
  (if (not (`self.IsRewinding`))
    (`self.K2_SetActorRotation` (`KismetMathLibrary.MakeRotator` (+ (* DeltaSeconds 200.0) _returnvalue_roll) _returnvalue_pitch _returnvalue_yaw))
    (set `self.TimeAccumulator` (+ DeltaSeconds (`self.TimeAccumulator`)))
    (if (>= (`self.TimeAccumulator`) 0.05)
      (if (>= (`KismetArrayLibrary.Array_Length` (`self.CurSnapshot`)) 500)
        (`KismetArrayLibrary.Array_Remove` (`self.CurSnapshot`)))
      (`KismetArrayLibrary.Array_Add` (`self.CurSnapshot`) (make `/Game/Blueprints/Character/ST_Snapshot` (`self.K2_GetActorLocation`) (`self.K2_GetActorRotation`) (struct)))
      (set `self.TimeAccumulator` 0.0))))

(event `/Game/Blueprints/Interfaces/BPI_Aimed.Aimed`
  (if (not (`self.IsFreezing`))
    (`PrimitiveComponent.SetCustomDepthStencilValue` (`self.StaticMesh`) 1)))

(event `/Game/Blueprints/Interfaces/BPI_ClearAim.ClearAim`
  (if (not (`self.IsFreezing`))
    (`PrimitiveComponent.SetCustomDepthStencilValue` (`self.StaticMesh`) 0)))

(event `/Game/Blueprints/Interfaces/BPI_TimeFreezing.TimeFreezing`
  (set `self.IsFreezing` true)
  (`PrimitiveComponent.SetCustomDepthStencilValue` (`self.StaticMesh`) 2)
  (`self.SetActorTickEnabled` false)
  (`KismetSystemLibrary.Delay` 3.0)
  (`PrimitiveComponent.SetCustomDepthStencilValue` (`self.StaticMesh`) 0)
  (`self.SetActorTickEnabled` true)
  (set `self.IsFreezing` false))

(event `/Game/Blueprints/Interfaces/BPI_TimeRewinding.TimeRewinding`
  (bind _cursnapshot (`self.CurSnapshot`))
  (bind _cursnapshot_2 (`self.CurSnapshot`))
  (bind (_output_location _output_rotation) (break `/Game/Blueprints/Character/ST_Snapshot` (`|GetArrayItem` _cursnapshot_2 (`KismetArrayLibrary.Array_LastIndex` _cursnapshot_2))))
  (set `self.IsRewinding` true)
  (if (`KismetArrayLibrary.Array_IsNotEmpty` (`self.CurSnapshot`))
    (`self.K2_SetActorLocationAndRotation` _output_location _output_rotation)
    (`KismetArrayLibrary.Array_Remove` _cursnapshot (`KismetArrayLibrary.Array_LastIndex` _cursnapshot))
    (set `self.IsRewinding` false)))

(fn `UserConstructionScript`)