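; BP_InvisibleFloor is an obstacle whose Cube stays hidden until the player's time gauge swings far enough in either direction.
; It starts invisible, then every Tick reads BP_ChronoHacker's TimeGauge and shows the Cube at or beyond a symmetric positive or negative threshold.
; Only visibility changes; collision is untouched.
; Time-ability query functions report it as freezable but not rewindable and expose IsFreezing, which the visibility logic ignores.
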(event `self.ReceiveBeginPlay`
  (`SceneComponent.SetVisibility` (`self.Cube`) false false))

(event `self.ReceiveTick`
  (params (DeltaSeconds :type "Float (single-precision)"))
  (bind _asbp_chrono_hacker (cast `/Game/Blueprints/Character/BP_ChronoHacker` (`GameplayStatics.GetPlayerCharacter` 0)))
  (bind (_mystat_maxhp _mystat_curhp _mystat_timegauge) (break `/Game/Blueprints/Character/ST_Stats` (`/Game/Blueprints/Character/BP_ChronoHacker.MyStat` _asbp_chrono_hacker)))
  (if (or (>= _mystat_timegauge 60.0) (>= -60.0 _mystat_timegauge))
    (`SceneComponent.SetVisibility` (`self.Cube`) true false)
    (else
      (`SceneComponent.SetVisibility` (`self.Cube`) false false))))

(fn `CanFreezing`
  (returns (CanFreezing :type Boolean))
  (return true))

(fn `CanRewinding`
  (returns (CanRewinding :type Boolean))
  (return false))

(fn `GetFreezingState`
  (returns (IsFreezing :type Boolean))
  (return (`self.IsFreezing`)))

(fn `UserConstructionScript`)