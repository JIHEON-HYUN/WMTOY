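; Crosshair component that manages aim spread for its owner and shows or hides the crosshair widget.
; A looping timer polls velocity to add movement and jump spread, which turns into recovering dynamic spread when that state ends.
; A spawned, attached helper actor supplies the timeline that drives recovery at a curve-based rate, with changes broadcast through OnSpreadChanged.
; Line-trace wrappers randomise end points by current spread, capped at MaxSpread.
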(event `self.ReceiveBeginPlay`
  (bind _returnvalue (`|SpawnActorFromClass` "/Game/Blueprints/CrosshairSystem/CT_Timeline_Crosshair.CT_Timeline_Crosshair_C" (`KismetMathLibrary.MakeTransform` (0.0 0.0 0.0)) "Undefined" "MultiplyWithRoot" (`self.GetOwner`) null))
  (set `self.Timeline` (`/Game/Blueprints/CrosshairSystem/CT_Timeline_Crosshair.Timeline` _returnvalue))
  (`Actor.K2_AttachToActor` _returnvalue (`self.GetOwner`) "None" "KeepRelative" "KeepRelative" "KeepRelative" true)
  (`KismetSystemLibrary.K2_SetTimer` null "HandleMove&FallSpread" 0.1 true))

(fn `AddDynamicSpread`
  (params (Spread :type "Float (double-precision)") (RecoveryRate :type "Float (double-precision)" :default 1.0))
  (locals (LocalAccuracy :type "Float (double-precision)" :default 0.0))
  (set `self.DynamicSpread` (+ (`self.DynamicSpread`) (`KismetMathLibrary.SelectFloat` (- (`self.MaxSpread`) (`self.GetSpreadValue`)) (`local.Spread`) (> (+ (`self.GetSpreadValue`) (`local.Spread`)) (`self.MaxSpread`)))))
  (`TimelineComponent.SetNewTime` (`self.Timeline`) (- 1.0 (`KismetMathLibrary.SafeDivide` (`self.DynamicSpread`) 1000.0)))
  (`TimelineComponent.Play` (`self.Timeline`))
  (`TimelineComponent.SetPlayRate` (`self.Timeline`) (* (/ (`self.DynamicSpread`) 1000.0) (/ 1.0 (`CurveFloat.GetFloatValue` (`self.SpreadRecoveryTimeCurve`) (`self.DynamicSpread`))) (`local.RecoveryRate`))))

(fn `GetCrossHairsWidget`
  (returns (ReturnValue :type "UserWidget Object Reference"))
  (locals (Local_Widget :type "UserWidget Object Reference"))
  (`|ExecutionSequence`
    (:`then_0`
      (bind _foundwidgets (`WidgetBlueprintLibrary.GetAllWidgetsOfClass` "/Game/Blueprints/CrosshairSystem/WBP_CrossHairs.WBP_CrossHairs_C"))
      (bind _output_get (set `local.Local_Widget` (`|GetArrayItem` _foundwidgets)))
      (`/Engine/EditorBlueprintResources/StandardMacros.IsValid` _output_get
        (:`Is Valid`
          (return (`local.Local_Widget`)))
        (:`Is Not Valid`
          (bind _ascharacter (cast `Character` (`self.GetOwner`)))
          (if (`Pawn.IsLocallyControlled` _ascharacter)
            (bind _returnvalue (`|CreateWidget` (`self.WidgetClass`) (`Pawn.GetLocalViewingPlayerController` _ascharacter)))
            (bind _output_get_2 (set `local.Local_Widget` _returnvalue))
            (`UserWidget.AddToViewport` _output_get_2 0)))))
    (:`then_1`
      (return (`local.Local_Widget`)))))

(fn `GetSpreadValue`
  (returns (ReturnValue :type "Float (double-precision)"))
  (return (`KismetMathLibrary.FMin` (+ (`self.DynamicSpread`) (`self.BaseSpread`) (`self.AdditionalSpread`)) (`self.MaxSpread`))))

(fn `GetTracePoint`
  (params (StartPoint :type "Transform Structure") (Distance :type "Float (double-precision)") (SpreadScale :type "Float (double-precision)" :default 1.0))
  (returns (Start :type "Vector Structure") (End :type "Vector Structure"))
  (bind _location (.location StartPoint))
  (return _location (+ (* (`KismetMathLibrary.GetForwardVector` (.rotation StartPoint)) (`local.Distance`)) (`KismetMathLibrary.RandomPointInBoundingBox` _location (* (* (* (`self.GetSpreadValue`) (`local.SpreadScale`)) (/ (`local.Distance`) (`self.CorrectionFactor`))) (1.0 1.0 1.0))))))

(fn `HandleMove&FallSpread`
  (`|ExecutionSequence`
    (:`then_0`
      (if (!= (`self.IsFalling`) (`self.LastFalling`))
        (bind _output_get (set `self.LastFalling` (not (`self.LastFalling`))))
        (if _output_get
          (set `self.AdditionalSpread` (+ (`self.AdditionalSpread`) (`self.JumpSpread`)))
          (`self.OnSpreadChanged` (`self.GetSpreadValue`))
          (else
            (set `self.AdditionalSpread` (- (`self.AdditionalSpread`) (`self.JumpSpread`)))
            (`self.AddDynamicSpread` (`self.JumpSpread`) (`self.SpreadRecoveryRate`))))))
    (:`then_1`
      (if (!= (`self.IsMoving`) (`self.LastMoving`))
        (bind _output_get_2 (set `self.LastMoving` (not (`self.LastMoving`))))
        (if _output_get_2
          (set `self.AdditionalSpread` (+ (`self.AdditionalSpread`) (`self.MovementSpread`)))
          (`self.OnSpreadChanged` (`self.GetSpreadValue`))
          (else
            (set `self.AdditionalSpread` (- (`self.AdditionalSpread`) (`self.MovementSpread`)))
            (`self.AddDynamicSpread` (`self.MovementSpread`) (`self.SpreadRecoveryRate`))))))))

(fn `HideCrossHairs`
  (locals (Local_Widget :type "UserWidget Object Reference"))
  (bind _output_get (set `local.Local_Widget` (`self.GetCrossHairsWidget`)))
  (`/Engine/EditorBlueprintResources/StandardMacros.IsValid` _output_get
    (:`Is Valid`
      (`Widget.SetVisibility` (`local.Local_Widget`) "Collapsed"))))

(fn `IsFalling`
  (returns (ReturnValue :type Boolean))
  (return (> (`KismetMathLibrary.Abs` (.z (`Actor.GetVelocity` (`self.GetOwner`)))) 0.0)))

(fn `IsMoving`
  (returns (ReturnValue :type Boolean))
  (return (> (`KismetMathLibrary.VSizeXY` (`Actor.GetVelocity` (`self.GetOwner`))) 0.0)))

(fn `LineTraceByChannel`
  (params (StartPoint :type "Transform Structure") (Distance :type "Float (double-precision)" :default 10000.0) (SpreadScale :type "Float (double-precision)" :default 1.0) (TraceChannel :type "ETraceTypeQuery Enum" :default "TraceTypeQuery1") (TraceComplex :type Boolean) (ActorsToIgnore :type "Array of Actor Object Reference (by ref)") (DrawDebugType :type "EDrawDebugTrace Enum" :default "None") (IgnoreSelf :type Boolean :default true))
  (returns (OutHit :type "HitResult Structure") (ReturnValue :type Boolean))
  (bind (_start _end) (`self.GetTracePoint` StartPoint Distance SpreadScale))
  (bind (_outhit _returnvalue) (`KismetSystemLibrary.LineTraceSingle` _start _end (`local.TraceChannel`) (`local.TraceComplex`) (`local.ActorsToIgnore`) (`local.DrawDebugType`) (`local.IgnoreSelf`)))
  (if _returnvalue
    (return _outhit _returnvalue)
    (else
      (return (`GameplayStatics.MakeHitResult` false false 0.0 0.0 (0.0 0.0 0.0) _end (0.0 0.0 1.0) _end) false))))

(fn `LineTraceByProfile`
  (params (StartPoint :type "Transform Structure") (Distance :type "Float (double-precision)" :default 10000.0) (SpreadScale :type "Float (double-precision)" :default 1.0) (ProfileName :type Name) (TraceComplex :type Boolean) (ActorsToIgnore :type "Array of Actor Object Reference (by ref)") (DrawDebugType :type "EDrawDebugTrace Enum" :default "None") (IgnoreSelf :type Boolean :default true))
  (returns (OutHit :type "HitResult Structure") (ReturnValue :type Boolean))
  (bind (_start _end) (`self.GetTracePoint` StartPoint Distance SpreadScale))
  (bind (_outhit _returnvalue) (`KismetSystemLibrary.LineTraceSingleByProfile` _start _end (`local.ProfileName`) (`local.TraceComplex`) (`local.ActorsToIgnore`) (`local.DrawDebugType`) (`local.IgnoreSelf`)))
  (if _returnvalue
    (return _outhit _returnvalue)
    (else
      (return (`GameplayStatics.MakeHitResult` false false 0.0 0.0 (0.0 0.0 0.0) _end (0.0 0.0 1.0) _end) false))))

(fn `LineTraceForObjects`
  (params (StartPoint :type "Transform Structure") (Distance :type "Float (double-precision)" :default 10000.0) (SpreadScale :type "Float (double-precision)" :default 1.0) (ObjectTypes :type "Array of EObjectTypeQuery Enum (by ref)") (TraceComplex :type Boolean) (ActorsToIgnore :type "Array of Actor Object Reference (by ref)") (DrawDebugType :type "EDrawDebugTrace Enum" :default "None") (IgnoreSelf :type Boolean :default true))
  (returns (OutHit :type "HitResult Structure") (ReturnValue :type Boolean))
  (bind (_start _end) (`self.GetTracePoint` StartPoint Distance SpreadScale))
  (bind (_outhit _returnvalue) (`KismetSystemLibrary.LineTraceSingleForObjects` _start _end (`local.ObjectTypes`) (`local.TraceComplex`) (`local.ActorsToIgnore`) (`local.DrawDebugType`) (`local.IgnoreSelf`)))
  (if _returnvalue
    (return _outhit _returnvalue)
    (else
      (return (`GameplayStatics.MakeHitResult` false false 0.0 0.0 (0.0 0.0 0.0) _end (0.0 0.0 1.0) _end) false))))

(fn `MultiLineTraceByChannel`
  (params (StartPoint :type "Transform Structure") (Distance :type "Float (double-precision)" :default 10000.0) (SpreadScale :type "Float (double-precision)" :default 1.0) (TraceChannel :type "ETraceTypeQuery Enum" :default "TraceTypeQuery1") (TraceComplex :type Boolean) (ActorsToIgnore :type "Array of Actor Object Reference (by ref)") (DrawDebugType :type "EDrawDebugTrace Enum" :default "None") (IgnoreSelf :type Boolean :default true))
  (returns (OutHit :type "Array of HitResult Structure") (ReturnValue :type Boolean))
  (bind (_start _end) (`self.GetTracePoint` StartPoint Distance SpreadScale))
  (bind (_outhits _returnvalue) (`KismetSystemLibrary.LineTraceMulti` _start _end (`local.TraceChannel`) (`local.TraceComplex`) (`local.ActorsToIgnore`) (`local.DrawDebugType`) (`local.IgnoreSelf`)))
  (if _returnvalue
    (return _outhits _returnvalue)
    (else
      (return false (`|MakeArray` (`GameplayStatics.MakeHitResult` false false 0.0 0.0 (0.0 0.0 0.0) _end (0.0 0.0 1.0) _end))))))

(fn `MultiLineTraceByProfile`
  (params (StartPoint :type "Transform Structure") (Distance :type "Float (double-precision)" :default 10000.0) (SpreadScale :type "Float (double-precision)" :default 1.0) (ProfileName :type Name) (TraceComplex :type Boolean) (ActorsToIgnore :type "Array of Actor Object Reference (by ref)") (DrawDebugType :type "EDrawDebugTrace Enum" :default "None") (IgnoreSelf :type Boolean :default true))
  (returns (OutHit :type "Array of HitResult Structure") (ReturnValue :type Boolean))
  (bind (_start _end) (`self.GetTracePoint` StartPoint Distance SpreadScale))
  (bind (_outhits _returnvalue) (`KismetSystemLibrary.LineTraceMultiByProfile` _start _end (`local.ProfileName`) (`local.TraceComplex`) (`local.ActorsToIgnore`) (`local.DrawDebugType`) (`local.IgnoreSelf`)))
  (if _returnvalue
    (return _outhits _returnvalue)
    (else
      (return false (`|MakeArray` (`GameplayStatics.MakeHitResult` false false 0.0 0.0 (0.0 0.0 0.0) _end (0.0 0.0 1.0) _end))))))

(fn `MultiLineTraceForObjects`
  (params (StartPoint :type "Transform Structure") (Distance :type "Float (double-precision)" :default 10000.0) (SpreadScale :type "Float (double-precision)" :default 1.0) (ObjectTypes :type "Array of EObjectTypeQuery Enum (by ref)") (TraceComplex :type Boolean) (ActorsToIgnore :type "Array of Actor Object Reference (by ref)") (DrawDebugType :type "EDrawDebugTrace Enum" :default "None") (IgnoreSelf :type Boolean :default true))
  (returns (OutHit :type "Array of HitResult Structure") (ReturnValue :type Boolean))
  (bind (_start _end) (`self.GetTracePoint` StartPoint Distance SpreadScale))
  (bind (_outhits _returnvalue) (`KismetSystemLibrary.LineTraceMultiForObjects` _start _end (`local.ObjectTypes`) (`local.TraceComplex`) (`local.ActorsToIgnore`) (`local.DrawDebugType`) (`local.IgnoreSelf`)))
  (if _returnvalue
    (return _outhits _returnvalue)
    (else
      (return false (`|MakeArray` (`GameplayStatics.MakeHitResult` false false 0.0 0.0 (0.0 0.0 0.0) _end (0.0 0.0 1.0) _end))))))

(fn `SetDefaultSpread`
  (params (Base :type "Float (double-precision)") (Jump :type "Float (double-precision)") (Movement :type "Float (double-precision)") (Max :type "Float (double-precision)" :default 1000.0))
  (locals (Local_BaseSpread :type "Float (double-precision)" :default 0.0))
  (set `self.MaxSpread` Max)
  (set `local.Local_BaseSpread` (`self.BaseSpread`))
  (`|ExecutionSequence`
    (:`then_0`
      (if (`self.LastFalling`)
        (set `self.AdditionalSpread` (- (`self.AdditionalSpread`) (`self.JumpSpread`)))
        (set `self.AdditionalSpread` (+ (`self.AdditionalSpread`) (`local.Jump`)))))
    (:`then_1`
      (if (`self.LastMoving`)
        (set `self.AdditionalSpread` (- (`self.AdditionalSpread`) (`self.MovementSpread`)))
        (set `self.AdditionalSpread` (+ (`self.AdditionalSpread`) (`local.Movement`)))))
    (:`then_2`
      (set `self.BaseSpread` (`local.Base`))
      (set `self.JumpSpread` (`local.Jump`))
      (set `self.MovementSpread` (`local.Movement`))
      (if (> (`local.Local_BaseSpread`) (`self.BaseSpread`))
        (`self.AddDynamicSpread` (- (`local.Local_BaseSpread`) (`self.BaseSpread`)) (`self.SpreadRecoveryRate`))
        (else
          (`self.OnSpreadChanged` (`self.GetSpreadValue`)))))))

(fn `ShowCrossHairs`
  (locals (Local_ :type "/Game/Blueprints/CrosshairSystem/WBP_CrossHairs Object Reference") (Local_Widget :type "UserWidget Object Reference"))
  (bind _output_get (set `local.Local_Widget` (`self.GetCrossHairsWidget`)))
  (`/Engine/EditorBlueprintResources/StandardMacros.IsValid` _output_get
    (:`Is Valid`
      (`Widget.SetVisibility` (`local.Local_Widget`) "Visible"))))

(fn `TryResetSpread`
  (`self.OnTryResetSpread`))

(fn `UpdateSpreadTimeline`
  (params (Direction :type "ETimelineDirection Enum" :default "Forward") (Value :type "Float (double-precision)"))
  (set `self.DynamicSpread` (* 1000.0 (`local.Value`)))
  (`self.OnSpreadChanged` (`self.GetSpreadValue`)))